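; Player pawn for a 2048 tile game that takes arrow-key input and drives the board through GM_Duri2048GameMode.
; BeginPlay caches the game mode and adds the WB_HUD widget to the viewport.
; Each arrow key shifts all four lines via MoveUpIndex or MoveDownIndex, spawning a new tile only if something moved.
; Debug keys spawn a tile or force a tile to 2048.
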(event `self.ReceiveBeginPlay`
  (bind _asgm_duri_2048game_mode (cast `/Game/Blueprints/GM_Duri2048GameMode` (`GameplayStatics.GetGameMode`)))
  (set `self.GameMode` _asgm_duri_2048game_mode)
  (bind _returnvalue (`|CreateWidget` "/Game/Blueprints/WB_HUD.WB_HUD_C"))
  (`UserWidget.AddToViewport` _returnvalue 0))

(event `Key|G`
  (params (Key :type "Key Structure"))
  ;[1 0.8165 0.3222] Debug
  (:`Pressed`
    (`Duri2048GameMode.GenerateTile` (`self.GameMode`))))

(event `Key|Right`
  (params (Key :type "Key Structure"))
  ;[1 1 1] Input Events
  (:`Pressed`
    (for _index (range 4)
      (bind _returnvalue (`Duri2048GameMode.MoveDownIndex` (`self.GameMode`) _index false))
      (if _returnvalue
        (set `self.bIsMove` true)))
    (if (`self.bIsMove`)
      (`Duri2048GameMode.GenerateTile` (`self.GameMode`))
      (set `self.bIsMove` false))))

(event `Key|W`
  (params (Key :type "Key Structure"))
  ;[1 0.8165 0.3222] Debug
  (:`Pressed`
    (bind _outactors (`GameplayStatics.GetAllActorsOfClass` "/Game/Blueprints/BP_Tile.BP_Tile_C"))
    (set `Tile.Number` 2048 (`|GetArrayItem` _outactors))
    (`Duri2048GameMode.GenerateTile` (`self.GameMode`))))

(event `Key|Left`
  (params (Key :type "Key Structure"))
  ;[1 1 1] Input Events
  (:`Pressed`
    (for _index (range 4)
      (bind _returnvalue (`Duri2048GameMode.MoveUpIndex` (`self.GameMode`) _index false))
      (if _returnvalue
        (set `self.bIsMove` true)))
    (if (`self.bIsMove`)
      (`Duri2048GameMode.GenerateTile` (`self.GameMode`))
      (set `self.bIsMove` false))))

(event `Key|Up`
  (params (Key :type "Key Structure"))
  ;[1 1 1] Input Events
  (:`Pressed`
    (for _index (range 4)
      (bind _returnvalue (`Duri2048GameMode.MoveDownIndex` (`self.GameMode`) _index true))
      (if _returnvalue
        (set `self.bIsMove` true)))
    (if (`self.bIsMove`)
      (`Duri2048GameMode.GenerateTile` (`self.GameMode`))
      (set `self.bIsMove` false))))

(event `Key|Down`
  (params (Key :type "Key Structure"))
  ;[1 1 1] Input Events
  (:`Pressed`
    (for _index (range 4)
      (bind _returnvalue (`Duri2048GameMode.MoveUpIndex` (`self.GameMode`) _index true))
      (if _returnvalue
        (set `self.bIsMove` true)))
    (if (`self.bIsMove`)
      (`Duri2048GameMode.GenerateTile` (`self.GameMode`))
      (set `self.bIsMove` false))))

(fn `UserConstructionScript`)