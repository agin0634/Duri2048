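; BP_ChessBoard lays out a 4x4 board of static meshes and spawns a matching grid of BP_Tile actors.
; The construction script adds one scaled mesh per cell, using integer division and modulo on the loop index for evenly spaced relative positions.
; BeginPlay repeats the grid math with a fixed offset to spawn the tiles in world space, independent of the board's own transform.
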(event `self.ReceiveBeginPlay`
  (for _index (range 16)
    (`|SpawnActorFromClass` "/Game/Blueprints/BP_Tile.BP_Tile_C" (`KismetMathLibrary.Conv_VectorToTransform` (+ (`KismetMathLibrary.MakeVector` (* (/ _index 4) 400.0) (* (mod _index 4) 400.0)) (180.0 180.0 25.0))) "Undefined" "OverrideRootScale" null null)))

(fn `UserConstructionScript`
  (for _index (range 16)
    (`AddComponent|NODE_AddStaticMeshComponent-0` :`RelativeTransform` (`KismetMathLibrary.MakeTransform` (`KismetMathLibrary.MakeVector` (* (/ _index 4) 400.0) (* (mod _index 4) 400.0)) (struct) (0.9 0.9 2.0)))))